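; BP_Decoration is a decoration actor that an SFPlayer can pick up by interacting with it.
; Interact asks the player whether pickup is allowed, then passes itself to PickupDecoration or prints a debug message.
; When BreakOnHit is set, a WorldModel hit plays a wood-break sound, spawns Niagara debris and destroys the actor.
; ChangeMaterial swaps the model's first material between picked-up and dropped looks.
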(event OnComponentHit(WorldModel)
  (params (HitComponent :type Primitive%20Component%20Object%20Reference) (OtherActor :type Actor%20Object%20Reference) (OtherComp :type Primitive%20Component%20Object%20Reference) (NormalImpulse :type Vector :default "0, 0, 0") (Hit :type Hit%20Result%20Structure%20%28by%20ref%29))
  (if (Variables|Default|GetBreakOnHit)
    (Class|SFDecoration|Break)
    (Niagara|SpawnSystematLocation "/Game/StoryForge/Niagara/NS_Debris.NS_Debris" (Transformation|GetActorLocation) (Transformation|GetActorRotation))
    (Actor|DestroyActor)))

(event EventBeginPlay)

(event Collision|EventActorBeginOverlap
  (params (OtherActor :type Actor%20Object%20Reference)))

(event EventTick
  (params (DeltaSeconds :type Float%20%28single-precision%29)))

(event EventInteract
  (params (CallingActor :type Actor%20Object%20Reference))
  (bind _assfplayer (Utilities|Casting|CastToSFPlayer CallingActor))
  (if (Class|SFPlayer|CanPickupDecoration _assfplayer)
    (Class|SFPlayer|PickupDecoration _assfplayer self)
    (else
      (Development|PrintString "cant pickup bruh"))))

(event EventBreak
  (Development|PrintString "Break")
  (Audio|PlaySoundatLocation "/Game/StoryForge/Audio/Raw/Physics/WoodBreakLarge.WoodBreakLarge" (Transformation|GetActorLocation) "0, 0, 0" 1.0 1.0 0.0 0 0 0 0))

(fn ConstructionScript)

(fn ChangeMaterial
  (params (PickedUp :type Boolean))
  (if PickedUp
    (LocalVariables|SetNewMaterial (Variables|Default|GetPickUpMaterial))
    (else
      (LocalVariables|SetNewMaterial (Variables|Default|GetDroppedMaterial))))
  (Rendering|Material|SetMaterial (Variables|Default|GetWorldModel) 0 (LocalVariables|GetNewMaterial)))