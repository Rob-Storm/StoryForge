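; Dialogue component that runs a conversation, tracking the current node as it begins, continues, jumps to an index or ends.
; Speech nodes link by next-node ID, and each newly entered node runs its pre-events, which post player messages or change camera angles.
; A spawned BP_DialogueCameras actor handles framing, while dispatcher calls broadcast dialogue and camera changes.
; Helpers run post-events, detect end nodes and control the GameMode's voice-line player.
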(fn BeginDialogue
  (params (Conversation :type Dialogue%20Asset%20Object%20Reference))
  (bind _initialcameraangle (Variables|/Script/StoryForge.DialogueAsset|GetInitialCameraAngle Conversation))
  (bind _cameraangle (Variables|/Script/StoryForge.DialogueEventCameraAngle|GetCameraAngle _initialcameraangle))
  (bind _target (Variables|/Script/StoryForge.DialogueEventCameraAngle|GetTarget _initialcameraangle))
  (bind _output (Utilities|ResolveSoftReference _target))
  (Variables|Dialogue|SetCurrentConversation Conversation)
  (Variables|Dialogue|SetInDialogue true)
  (bind _output_get (Variables|Dialogue|SetCurrentDialogueIndex 0))
  (bind _output_get_2 (Variables|Dialogue|SetCurrentDialogueNode (Utilities|Array|Get(acopy) (Variables|/Script/StoryForge.DialogueAsset|GetDialogueNodes (Variables|Dialogue|GetCurrentConversation)) _output_get)))
  (Dialogue|RunPreEvents _output_get_2)
  (Default|CallOnBeginDialogue Conversation)
  (bind _returnvalue (Game|SpawnActorfromClass "/Game/StoryForge/Blueprints/Dialogue/BP_DialogueCameras.BP_DialogueCameras_C" (Transformation|GetActorTransform _output) "AlwaysSpawn" "MultiplyWithRoot" 0 0))
  (bind _output_get_3 (Variables|Dialogue|SetDialogueCameras _returnvalue))
  (if (Variables|/Script/StoryForge.DialogueEventCameraAngle|GetTargetIsPlayer _initialcameraangle)
    (bind _cameratransform (Default|SetCameraRotation _output_get_3 _cameraangle (Game|Player|GetPlayerPawn 0)))
    (Default|CallOnChangeCamera _cameratransform)
    (else
      (bind _cameratransform_2 (Default|SetCameraRotation _output_get_3 _cameraangle _output))
      (Default|CallOnChangeCamera _cameratransform_2))))

(fn ContinueDialogue
  (Class|KismetSystemLibrary|IsObjectOfSoftClass (Variables|Dialogue|GetCurrentDialogueNode) "/Script/StoryForge.DialogueNodeEnd"
    (:True
      (Dialogue|EndDialogue))
    (:False
      (bind _asdialogue_node_speech (Utilities|Casting|CastToDialogueNodeSpeech (Variables|Dialogue|GetCurrentDialogueNode))
        (:then
          (bind _output_get (Variables|Dialogue|SetCurrentDialogueNode (Utilities|Array|Get(acopy) (Variables|/Script/StoryForge.DialogueAsset|GetDialogueNodes (Variables|Dialogue|GetCurrentConversation)) (Variables|/Script/StoryForge.DialogueNodeSpeech|GetNextNodeId _asdialogue_node_speech))))
          (Dialogue|RunPreEvents _output_get)
          (Default|CallOnDialogueContinue _output_get))
        (:CastFailed
          (return))))))

(fn JumptoNode
  (params (NodeIndex :type Integer))
  (bind _currentconversation (Variables|Dialogue|GetCurrentConversation))
  (bind _dialoguenodes (Variables|/Script/StoryForge.DialogueAsset|GetDialogueNodes _currentconversation))
  (bind _output (Utilities|Array|Get(acopy) _dialoguenodes NodeIndex))
  (Utilities|IsValid _output
    (:Is%20Valid
      (bind _output_get (Variables|Dialogue|SetCurrentDialogueNode _output))
      (Dialogue|RunPreEvents _output_get)
      (Default|CallOnDialogueJump _output_get))
    (:Is%20Not%20Valid
      (Dialogue|EndDialogue))))

(fn EndDialogue
  (Variables|Dialogue|SetInDialogue false)
  (Variables|Dialogue|SetCurrentConversation 0)
  (Variables|Dialogue|SetCurrentDialogueNode 0)
  (Variables|Dialogue|SetCurrentDialogueIndex -1)
  (Default|CallOnDialogueEnd))

(fn RunEvents
  (params (Events :type Array%20of%20Dialogue%20Node%20Event%20Object%20References))
  (bind _dialoguecameras (Variables|Dialogue|GetDialogueCameras))
  (if (>= (Utilities|Array|Length Events) 0)
    (for _array_element Events
      (Development|PrintString (Utilities|GetDisplayName _array_element))
      (bind _asdialogue_event_client_message (Utilities|Casting|CastToDialogueEventClientMessage _array_element)
        (:then
          (bind _asbp_player (Utilities|Casting|CastToBP_Player (Game|Player|GetPlayerPawn 0)))
          (Default|AddClientMessage _asbp_player (Variables|/Script/StoryForge.DialogueEventClientMessage|GetClientMessage _asdialogue_event_client_message)))
        (:CastFailed
          (bind _asdialogue_event_camera_angle (Utilities|Casting|CastToDialogueEventCameraAngle _array_element))
          (if (Variables|/Script/StoryForge.DialogueEventCameraAngle|GetTargetIsPlayer _asdialogue_event_camera_angle)
            (bind _cameratransform (Default|SetCameraRotation _dialoguecameras (Variables|/Script/StoryForge.DialogueEventCameraAngle|GetCameraAngle _asdialogue_event_camera_angle) (Game|Player|GetPlayerPawn 0)))
            (Default|CallOnChangeCamera _cameratransform)
            (else
              (bind _cameratransform_2 (Default|SetCameraRotation _dialoguecameras (Variables|/Script/StoryForge.DialogueEventCameraAngle|GetCameraAngle _asdialogue_event_camera_angle) (Utilities|ResolveSoftReference (Variables|/Script/StoryForge.DialogueEventCameraAngle|GetTarget _asdialogue_event_camera_angle))))
              (Default|CallOnChangeCamera _cameratransform_2)))))))
  (return))

(fn RunPreEvents
  (params (Node :type Dialogue%20Node%20Object%20Reference))
  (Dialogue|RunEvents (Variables|/Script/StoryForge.DialogueNode|GetPreEvents Node)))

(fn RunPostEvents
  (params (Node :type Dialogue%20Node%20Object%20Reference))
  (Dialogue|RunEvents (Variables|/Script/StoryForge.DialogueNode|GetPostEvents Node)))

(fn IsNodeEnd
  (params (Node :type Dialogue%20Node%20Object%20Reference))
  (return (Class|GameplayStatics|ObjectIsA Node "/Script/StoryForge.DialogueNodeEnd")))

(fn IsNextNodeEnd
  (params (CurrentNode :type Dialogue%20Node%20Object%20Reference))
  (LocalVariables|SetDialogueNodes (Variables|/Script/StoryForge.DialogueAsset|GetDialogueNodes (Variables|Dialogue|GetCurrentConversation)))
  (bind _asdialogue_node_speech (Utilities|Casting|CastToDialogueNodeSpeech CurrentNode))
  (return (Dialogue|IsNodeEnd (Utilities|Array|Get(acopy) (LocalVariables|GetDialogueNodes) (Variables|/Script/StoryForge.DialogueNodeSpeech|GetNextNodeId _asdialogue_node_speech))) (Variables|/Script/StoryForge.DialogueNodeSpeech|GetNextNodeId _asdialogue_node_speech)))

(fn PlayVoiceLine
  (params (VoiceClip :type Sound%20Base%20Object%20Reference))
  (bind _gamemoderef (Variables|Dialogue|GetGameModeRef))
  (bind _voicelineplayer (Variables|/Game/StoryForge/Core/BPGM_Game.BPGM_Game_C|GetVoiceLinePlayer _gamemoderef))
  (Audio|Components|Audio|SetSound _voicelineplayer VoiceClip)
  (Audio|Components|Audio|Play _voicelineplayer 0.0))

(fn StopVoiceLine
  (Audio|Components|Audio|Stop (Variables|/Game/StoryForge/Core/BPGM_Game.BPGM_Game_C|GetVoiceLinePlayer (Variables|Dialogue|GetGameModeRef))))