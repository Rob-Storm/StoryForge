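; Dialogue camera rig actor holding six preset shot cameras, from side and head shots to high and low angles.
; ChangeCameraAngle deactivates all cameras, then activates the one matching the chosen angle.
; SetCameraRotation snaps the rig to the target's transform, raised slightly for SFCharacter targets, switches angle, prints a debug string and returns that camera's world transform.
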(event EventBeginPlay
  (Variables|Default|SetCameras (Utilities|Array|MakeArray (Variables|Default|GetSideTight) (Variables|Default|GetSideMid) (Variables|Default|GetAboveDown) (Variables|Default|GetBelowUp) (Variables|Default|GetHeadShotTight) (Variables|Default|GetHeadShotMid))))

(fn ConstructionScript)

(fn ResetCameras
  (for _array_element (Variables|Default|GetCameras)
    (Components|Activation|SetActive _array_element false false)))

(fn ChangeCameraAngle
  (params (Selection :type ECameraAngle%20Enum :default "SideTight"))
  (CallFunction|ResetCameras)
  (switch Utilities|FlowControl|Switch|SwitchonECameraAngle Selection
    (:SideTight
      (Components|Activation|SetActive (Variables|Default|GetSideTight) true false))
    (:SideMid
      (Components|Activation|SetActive (Variables|Default|GetSideMid) true false))
    (:AboveDown
      (Components|Activation|SetActive (Variables|Default|GetAboveDown) true false))
    (:BelowUp
      (Components|Activation|SetActive (Variables|Default|GetBelowUp) true false))
    (:HeadTight
      (Components|Activation|SetActive (Variables|Default|GetHeadShotTight) true false))
    (:HeadMid
      (Components|Activation|SetActive (Variables|Default|GetHeadShotMid) true false))))

(fn GetCameraTransform
  (params (Selection :type ECameraAngle%20Enum :default "SideTight"))
  (switch Utilities|FlowControl|Switch|SwitchonECameraAngle Selection
    (:SideTight
      (return (Transformation|GetWorldTransform (Variables|Default|GetSideTight))))
    (:SideMid
      (return (Transformation|GetWorldTransform (Variables|Default|GetSideMid))))
    (:AboveDown
      (return (Transformation|GetWorldTransform (Variables|Default|GetAboveDown))))
    (:BelowUp
      (return (Transformation|GetWorldTransform (Variables|Default|GetBelowUp))))
    (:HeadTight
      (return (Transformation|GetWorldTransform (Variables|Default|GetHeadShotTight))))
    (:HeadMid
      (return (Transformation|GetWorldTransform (Variables|Default|GetHeadShotMid))))))

(fn SetCameraRotation
  (params (CameraAngle :type ECameraAngle%20Enum :default "SideTight") (Target :type Actor%20Object%20Reference))
  (bind _returnvalue (Transformation|GetActorTransform Target))
  (bind (_location _rotation _scale) (Math|Transform|BreakTransform _returnvalue))
  (Utilities|Casting|CastToSFCharacter Target
    (:then
      (Transformation|SetActorTransform (Math|Transform|MakeTransform (+ _location "0.000000,0.000000,70.000000") _rotation _scale)))
    (:CastFailed
      (Transformation|SetActorTransform _returnvalue)))
  (CallFunction|ChangeCameraAngle CameraAngle)
  (Development|PrintString (Utilities|String|Append "Angle: " (Utilities|String|EnumtoString CameraAngle) "    Target: " (Utilities|GetDisplayName Target)))
  (return (CallFunction|GetCameraTransform CameraAngle)))