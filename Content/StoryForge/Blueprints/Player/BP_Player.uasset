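; BP_Player is the first-person player character, handling Enhanced Input movement, sprint, jump, interaction, the inventory menu and on-screen client messages.
; A short camera line trace finds Interactable actors, driving both the interact action and a per-tick highlight box fitted to screen bounds.
; Game mode dialogue events switch to a repositionable dialogue camera, while death plays music and activates a rotating death camera.
; Picked-up decorations attach to HoldPoint with physics, collision off and a swapped material.
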(event Custom|OnBeginDialogue_Event
  (params (DialogueAsset :type Dialogue%20Asset%20Object%20Reference))
  (Components|Activation|SetActive (Variables|Default|GetCamera) false false)
  (Components|Activation|SetActive (Variables|Default|GetDialogueCamera) true false)
  (Class|PrimitiveComponent|SetOwnerNoSee (Variables|Character|GetMesh) false)
  (Components|Movement|StopMovementImmediately (Variables|Character|GetCharacterMovement)))

(event Custom|OnDialogueEnd_Event
  (Components|Activation|SetActive (Variables|Default|GetCamera) true false)
  (Components|Activation|SetActive (Variables|Default|GetDialogueCamera) false false)
  (Class|PrimitiveComponent|SetOwnerNoSee (Variables|Character|GetMesh) true))

(event Custom|OnChangeCamera_Event
  (params (NewTransform :type Transform))
  (Transformation|SetWorldTransform (Variables|Default|GetDialogueCamera) NewTransform false false))

(event EventBeginPlay
  (bind _returnvalue (UserInterface|CreateWidget "/Game/StoryForge/Widgets/Game/Interactable/WBP_InteractableBox.WBP_InteractableBox_C" (Game|GetPlayerController 0)))
  (bind _output_get (Variables|Default|SetInteractablePanel _returnvalue))
  (UserInterface|Viewport|AddtoViewport _output_get 0)
  (bind _returnvalue_2 (UserInterface|CreateWidget "/Game/StoryForge/Widgets/Game/Log/WBP_MessageHolder.WBP_MessageHolder_C" (Game|GetPlayerController 0)))
  (Variables|Default|SetClientMessages _returnvalue_2)
  (UserInterface|Viewport|AddtoViewport _returnvalue_2 0)
  (bind _asbpgm_game (Utilities|Casting|CastToBPGM_Game (Game|GetGameMode)))
  (EventDispatchers|AssignOnBeginDialogue (Variables|/Game/StoryForge/Core/BPGM_Game.BPGM_Game_C|GetBP_DialogueComponent _asbpgm_game) (delegate Custom|OnBeginDialogue_Event))
  (EventDispatchers|AssignOnDialogueEnd (Variables|/Game/StoryForge/Core/BPGM_Game.BPGM_Game_C|GetBP_DialogueComponent _asbpgm_game) (delegate Custom|OnDialogueEnd_Event))
  (EventDispatchers|AssignOnChangeCamera (Variables|/Game/StoryForge/Core/BPGM_Game.BPGM_Game_C|GetBP_DialogueComponent _asbpgm_game) (delegate Custom|OnChangeCamera_Event)))

(event EventAddClientMessage
  (params (ClientMessage :type Client%20Message%20Structure))
  (Default|AddClientMessage (Variables|Default|GetClientMessages) ClientMessage))

(event EventTick
  (params (DeltaSeconds :type Float%20%28single-precision%29))
  (bind _deathcamera (Variables|Default|GetDeathCamera))
  (Utilities|FlowControl|Sequence
    (:then_0
      (if (Components|Activation|IsActive _deathcamera)
        (Transformation|AddLocalRotation _deathcamera (* (Math|Rotator|MakeRotator 2e+01 0.0 0.0) DeltaSeconds) false false)))
    (:then_1
      (CallFunction|CheckInfoPanel))))

(event EventDie
  (bind _asplayer_controller (Utilities|Casting|CastToPlayerController (Pawn|GetController)))
  (Variables|/Script/Engine.PlayerController|SetbShowMouseCursor _asplayer_controller true)
  (Input|SetInputModeUIOnly _asplayer_controller 0 "DoNotLock" true)
  (Class|PrimitiveComponent|SetOwnerNoSee (Variables|Character|GetMesh) false)
  (bind _asbpgm_game (Utilities|Casting|CastToBPGM_Game (Game|GetGameMode)))
  (Default|ChangeMusicTracks _asbpgm_game "Death" false)
  (|CallParentFunction)
  (Utilities|FlowControl|Delay 1.5)
  (Components|Activation|Deactivate (Variables|Default|GetCamera))
  (Components|Activation|Activate (Variables|Default|GetDeathCamera) false))

(fn ConstructionScript
  (|CallParentFunction))

(fn Suicide
  (Class|SFCharacter|Die))

(fn InteractTrace
  (params (DrawDebugType :type EDrawDebugTrace%20Enum :default "None"))
  (bind _camera (Variables|Default|GetCamera))
  (bind _returnvalue (Transformation|GetWorldLocation _camera))
  (bind _outhit (Collision|LineTraceByChannel _returnvalue (+ _returnvalue (* (Math|Vector|GetForwardVector _camera) 300)) "TraceTypeQuery1" false 0 DrawDebugType true "(R=1.000000,G=0.000000,B=0.000000,A=1.000000)" "(R=0.000000,G=1.000000,B=0.000000,A=1.000000)" 2.0))
  (if (Utilities|DoesObjectImplementInterface (.hitactor _outhit) "/Script/StoryForge.Interactable")
    (return (.hitactor _outhit) true)
    (else
      (return 0 false))))

(fn PickupDecoration
  (params (DecorationActor :type SF%20Decoration%20Object%20Reference))
  (bind _output_get (Variables|Default|SetHeldDecoration DecorationActor))
  (Physics|SetSimulatePhysics (Variables|/Script/StoryForge.SFDecoration|GetWorldModel _output_get) false)
  (bind _returnvalue (Rendering|Material|CreateDynamicMaterialInstance (Variables|/Script/StoryForge.SFDecoration|GetWorldModel _output_get) 0 (Rendering|Material|GetMaterial (Variables|/Script/StoryForge.SFDecoration|GetWorldModel _output_get) 0) "None" :!class /Script/Engine.PrimitiveComponent))
  (bind _returnvalue_2 (Rendering|Material|GetTextureParameterValue _returnvalue "Texture" :!class /Script/Engine.MaterialInstanceDynamic))
  (bind _output_get_2 (LocalVariables|SetObjectTexture _returnvalue_2))
  (bind _returnvalue_3 (Rendering|Material|CreateDynamicMaterialInstance "/Game/StoryForge/Materials/M_ObjectTexture.M_ObjectTexture" "None" "None" :!class /Script/Engine.KismetMaterialLibrary))
  (Rendering|Material|SetTextureParameterValue _returnvalue_3 "Texture" _output_get_2)
  (Rendering|Material|SetMaterial (Variables|/Script/StoryForge.SFDecoration|GetWorldModel DecorationActor) 0 _returnvalue_3)
  (Transformation|AttachComponentToComponent (Variables|Default|GetHeldDecoration) (Variables|Default|GetHoldPoint) "None" "SnapToTarget" "KeepWorld" "KeepWorld" true)
  (Collision|SetCollisionEnabled (Variables|/Script/StoryForge.SFDecoration|GetWorldModel (Variables|Default|GetHeldDecoration)) "NoCollision"))

(fn CheckInfoPanel
  (bind _interactablepanel (Variables|Default|GetInteractablePanel))
  (bind (_interactable _returnhit) (CallFunction|InteractTrace "None"))
  (LocalVariables|SetActor _interactable)
  (if _returnhit
    (Widget|SetVisibility _interactablepanel "Visible")
    (bind (_outscreenposition _outscreensize) (Class|SFPlayer|GetActorBoundsasScreenCoords (LocalVariables|GetActor) (Game|GetPlayerController 0) 1.25))
    (Class|UserWidget|SetPositioninViewport (Variables|Default|GetInteractablePanel) _outscreenposition true)
    (Default|SetSize (Variables|Default|GetInteractablePanel) _outscreensize)
    (else
      (Widget|SetVisibility _interactablepanel "Collapsed"))))

(event Input|EnhancedActionEvents|EnhancedInputActionIA_Look
  (params (ActionValue :type Vector%202D%20Structure) (ElapsedSeconds :type Float%20%28double-precision%29) (TriggeredSeconds :type Float%20%28double-precision%29) (InputAction :type Input%20Action%20Object%20Reference :default "/Game/StoryForge/Input/Game/Actions/IA_Look.IA_Look"))
  (Pawn|Input|AddControllerYawInput (.x ActionValue))
  (Pawn|Input|AddControllerPitchInput (* (.y ActionValue) -1.0)))

(event Input|EnhancedActionEvents|EnhancedInputActionIA_Move
  (params (ActionValue :type Vector%202D%20Structure) (ElapsedSeconds :type Float%20%28double-precision%29) (TriggeredSeconds :type Float%20%28double-precision%29) (InputAction :type Input%20Action%20Object%20Reference :default "/Game/StoryForge/Input/Game/Actions/IA_Move.IA_Move"))
  (Pawn|Input|AddMovementInput (Transformation|GetActorRightVector) (.x ActionValue) false)
  (Pawn|Input|AddMovementInput (Transformation|GetActorForwardVector) (.y ActionValue) false))

(event Input|EnhancedActionEvents|EnhancedInputActionIA_Sprint
  (params (ActionValue :type Boolean) (ElapsedSeconds :type Float%20%28double-precision%29) (TriggeredSeconds :type Float%20%28double-precision%29) (InputAction :type Input%20Action%20Object%20Reference :default "/Game/StoryForge/Input/Game/Actions/IA_Sprint.IA_Sprint"))
  (bind _charactermovement (Variables|Character|GetCharacterMovement))
  (:Started
    (Variables|/Script/Engine.CharacterMovementComponent|SetMaxWalkSpeed _charactermovement (Variables|Default|GetRunSpeed)))
  (:Canceled
    (Variables|/Script/Engine.CharacterMovementComponent|SetMaxWalkSpeed _charactermovement (Variables|Default|GetWalkSpeed) :!label _label))
  (:Completed
    (goto _label)))

(event Input|EnhancedActionEvents|EnhancedInputActionIA_Jump
  (params (ActionValue :type Boolean) (ElapsedSeconds :type Float%20%28double-precision%29) (TriggeredSeconds :type Float%20%28double-precision%29) (InputAction :type Input%20Action%20Object%20Reference :default "/Game/StoryForge/Input/Game/Actions/IA_Jump.IA_Jump"))
  (:Started
    (Character|Jump))
  (:Canceled
    (Character|StopJumping :!label _label))
  (:Completed
    (goto _label)))

(event Input|EnhancedActionEvents|EnhancedInputActionIA_Interact
  (params (ActionValue :type Boolean) (ElapsedSeconds :type Float%20%28double-precision%29) (TriggeredSeconds :type Float%20%28double-precision%29) (InputAction :type Input%20Action%20Object%20Reference :default "/Game/StoryForge/Input/Game/Actions/IA_Interact.IA_Interact"))
  (:Started
    (bind (_interactable _returnhit) (CallFunction|InteractTrace "ForDuration"))
    (if _returnhit
      (Class|Interactable|Interact(Message) _interactable self))))

(event Input|EnhancedActionEvents|EnhancedInputActionIA_Inventory
  (params (ActionValue :type Boolean) (ElapsedSeconds :type Float%20%28double-precision%29) (TriggeredSeconds :type Float%20%28double-precision%29) (InputAction :type Input%20Action%20Object%20Reference :default "/Game/StoryForge/Input/Game/Actions/IA_Inventory.IA_Inventory"))
  (bind _returnvalue (Game|GetPlayerController 0))
  (:Started
    (bind _returnvalue_2 (UserInterface|CreateWidget "/Game/StoryForge/Widgets/Game/Menus/WBP_UserMenu.WBP_UserMenu_C" _returnvalue (Variables|Default|GetInventoryComponent)))
    (UserInterface|Viewport|AddtoViewport _returnvalue_2 0)
    (Input|SetInputModeUIOnly _returnvalue _returnvalue_2 "DoNotLock" true)
    (Variables|/Script/Engine.PlayerController|SetbShowMouseCursor _returnvalue true)
    (Game|SetGamePaused false)))